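; BP_P38 is a player-controlled P-38 plane that constantly flies forward and fires rockets.
; Tick spins the Left and Right propellers and feeds forward movement input scaled by Boost, which the boost action sets lower while held.
; Roll and Pitch axes rotate the actor locally, reusing the propeller rotation speed as the turn rate.
; Fire spawns a BP_rocket at the Arrow component's world transform.
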(event EventBeginPlay)

(event Collision|EventActorBeginOverlap
  (params (OtherActor :type Actor%20Object%20Reference)))

(event EventTick
  (params (DeltaSeconds :type Float%20%28single-precision%29))
  ;[1 1 1] 왼.프 회
  (Transformation|AddLocalRotation (Variables|Default|Getleft) (Math|Rotator|MakeRotator (* (Utilities|Time|GetWorldDeltaSeconds) (Variables|Default|GetPropellerRotateSpeed)) 0.0 0.0) false false)
  ;[1 1 1] 오.프 회
  (Transformation|AddLocalRotation (Variables|Default|GetRight) (Math|Rotator|MakeRotator (* (Utilities|Time|GetWorldDeltaSeconds) (Variables|Default|GetPropellerRotateSpeed)) 0.0 0.0) false false)
  ;[1 1 1] 이동
  (Pawn|Input|AddMovementInput (Transformation|GetActorForwardVector) (Variables|Default|Getboost) false))

(event Input|ActionEvents|InputActionboost
  (params (Key :type Key%20Structure :default "None"))
  (:Pressed
    ;[1 1 1] 부스트
    (Variables|Default|Setboost 0.5))
  (:Released
    (Variables|Default|Setboost 1.0)))

(event Input|ActionEvents|InputActionFire
  (params (Key :type Key%20Structure :default "None"))
  (:Pressed
    ;[1 1 1] 로켓생성
    (Game|SpawnActorfromClass "/Game/P38/Bluprints/BP_rocket.BP_rocket_C" (Transformation|GetWorldTransform (Variables|Default|GetArrow)) "Undefined" 0 0)))

(event Input|AxisEvents|InputAxisRoll
  (params (AxisValue :type Float%20%28single-precision%29))
  ;[1 1 1] 롤이동
  (Transformation|AddActorLocalRotation (Math|Rotator|MakeRotator (* AxisValue (Utilities|Time|GetWorldDeltaSeconds) (Variables|Default|GetPropellerRotateSpeed)) 0.0 0.0) false false))

(event Input|AxisEvents|InputAxisPitch
  (params (AxisValue :type Float%20%28single-precision%29))
  ;[1 1 1] 피치이동
  (Transformation|AddActorLocalRotation (Math|Rotator|MakeRotator 0.0 (* AxisValue (Utilities|Time|GetWorldDeltaSeconds) (Variables|Default|GetPropellerRotateSpeed)) 0.0) false false))

(fn ConstructionScript)